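; BP_BaseNPC is a base NPC that wanders randomly and can be sent to eat at a given destination or actor.
; From BeginPlay it loops AI MoveTo calls to random reachable points around itself, pausing briefly after each arrival.
; NPCEat sets an Eat flag that stops the loop rescheduling, moves to the target, waits, then resumes wandering and clears the flag.
; Only successful moves are handled, so a failed move continues neither sequence.
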(event `self.ReceiveBeginPlay`
  (`self.NPC Start Walking`))

(event `NPC Start Walking`
  (`|AIMoveTo` self (`NavigationSystemV1.K2_GetRandomReachablePointInRadius` (`self.K2_GetActorLocation`) 2000.0 null null) null
    (:`OnSuccess`
      (`KismetSystemLibrary.Delay` 2.0)
      (if (not (`self.Eat`))
        (`self.NPC Start Walking`)))))

(event `NPC Eat`
  (params (Destination :type "Vector Structure") (TargetActor :type "Actor Object Reference"))
  (set `self.Eat` true)
  (`|AIMoveTo` self Destination TargetActor
    (:`OnSuccess`
      (`KismetSystemLibrary.Delay` 5.0)
      (`self.NPC Start Walking`)
      (set `self.Eat` false))))

(fn `UserConstructionScript`)