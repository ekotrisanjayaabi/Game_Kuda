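; Feeding-point actor that sends horse NPCs of a given HorseType to eat at it.
; EatNPC checks the HorseType, then loops over the ActorOfHorse array and calls NPCEat on each matching horse, passing the Cube's world location as destination and itself as target.
; BeginPlay, Tick and overlap events are empty, so it acts only when EatNPC is called.
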(event `self.ReceiveBeginPlay`)

(event `Eat NPC`
  (params (`Horse Type` :type "/Game/_Main/Enum/E_HorseType Enum" :default "NewEnumerator0"))
  (if (`|EnumEquality` (`self.Horse Type`) `Horse Type`)
    (for _array_element (`self.Actor of Horse`)
      (if (`|EnumEquality` (`self.Horse Type`) (`/Game/_Main/Blueprints/BP_BaseNPC.Horse Type` _array_element))
        (`/Game/_Main/Blueprints/BP_BaseNPC.NPC Eat` _array_element (`SceneComponent.K2_GetComponentLocation` (`self.Cube`)) self)))))

(fn `UserConstructionScript`)